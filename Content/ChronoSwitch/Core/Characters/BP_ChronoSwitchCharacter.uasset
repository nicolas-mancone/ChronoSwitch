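; Player character Blueprint for ChronoSwitch, handling animation, audio and cosmetic feedback for switching between past and future timelines.
; A switch montage's notify fires the switch logic.
; Locally controlled timeline changes set flash visuals and MetaSound cues, with a reversible Timeline driving the MC_TimeSwap parameter collection and soundscape crossfade.
; It also handles visor fades, movement sounds, anti-phasing error audio, multicast mesh swaps and a debug Q visor toggle.
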(event `Multicast_ChangeCharacter`
  (params (SkeletalMesh :type "SkeletalMesh Object Reference") (AnimBP :type "AnimInstance Class Reference"))
  (`SkeletalMeshComponent.SetSkeletalMeshAsset` (`self.Mesh`) SkeletalMesh)
  (`SkeletalMeshComponent.SetAnimInstanceClass` (`self.Mesh`) AnimBP))

(event `self.OnJumped`
  (`AudioComponent.Play` (`self.MS_Jump`) 0.0))

(event `self.OnLanded`
  (params (Hit :type "HitResult Structure (by ref)"))
  (bind (_velocity_x _velocity_y _velocity_z) (`KismetMathLibrary.BreakVector` (`MovementComponent.Velocity` (`self.CharacterMovement`))))
  (if (< _velocity_z -100.0)
    (`AudioComponent.Play` (`self.MSS_Land`) 0.0)))

(event `self.ReceiveBeginPlay`
  ;[0 0.3713 1 0.5] BeginPlay
  (`self.SetupSounds`)
  (if (`self.IsLocallyControlled`)
    _))

(event `EnhancedInput|/Game/ChronoSwitch/Core/Input/InputActions/IA_Move`
  (params (ActionValue :type "Vector2D Structure") (ElapsedSeconds :type "Float (double-precision)") (TriggeredSeconds :type "Float (double-precision)") (InputAction :type "InputAction Object Reference" :default "/Game/ChronoSwitch/Core/Input/InputActions/IA_Move.IA_Move"))
  (bind _ms_footsteps (`self.MS_Footsteps`))
  (bind _returnvalue (`NavMovementComponent.IsFalling` (`self.CharacterMovement`)))
  (:`Triggered`
    (bind _output_get (set `self.IsMoving` true))
    (`AudioParameterControllerInterface.SetBoolParameter` _ms_footsteps "IsMoving" _output_get)
    (`AudioParameterControllerInterface.SetBoolParameter` _ms_footsteps "IsJumping" _returnvalue))
  (:`Canceled`
    (bind _output_get_2 (set `self.IsMoving` false :!label _label))
    (`AudioParameterControllerInterface.SetBoolParameter` _ms_footsteps "IsMoving" _output_get_2)
    (`AudioParameterControllerInterface.SetBoolParameter` _ms_footsteps "IsJumping" _returnvalue))
  (:`Completed`
    (goto _label)))

(event `self.OnTimeSwitchPressed`
  ;[1 0.4517 0 0.5] Switch Animation
  (`/Engine/EditorBlueprintResources/StandardMacros.DoOnce` false :!label _label_2
    (:`Completed`
      (bind _notifyname (`|PlayMontage` (`self.Mesh`) (select `bool` (`self.bIsPlayer1`) :`false` "/Game/ChronoSwitch/Characters/Taylor/AM_Switch.AM_Switch" :`true` "/Game/ChronoSwitch/Characters/John/Animations/AM_Switch.AM_Switch" :!type "AnimMontage Object Reference"))
        (:`OnCompleted`
          (goto _label_2 :!via `Reset`))
        (:`OnInterrupted`
          (goto _label_2 :!via `Reset`))
        (:`OnNotifyBegin`
          (switch `name` _notifyname
            (:`switch`
              (`AudioComponent.Play` (`self.MS_SwitchClick`) 0.0)
              (`self.ExecuteTimeSwitchLogic`))))
        (:`OnNotifyEnd`
          (goto _label_2 :!via `Reset`))))))

(event `self.OnTimelineChangedCosmetic`
  (params (NewTimelineID :type Byte))
  (bind _ms_switch (`self.MS_Switch`))
  (bind _parametervalue (`self.ParameterValue`))
  (bind _ms_soundscape (`self.MS_Soundscape`))
  ;[0 0.3713 1 0.5] Handle Timeline Switch Cosmetic Effects
  (if (`self.IsLocallyControlled`)
    (if (== NewTimelineID 1)
      (`KismetMaterialLibrary.SetVectorParameterValue` "/Game/ChronoSwitch/Materials/Collections/MC_TimeSwap.MC_TimeSwap" "FlashColor" (`|GetArrayItem` _parametervalue))
      (`KismetMaterialLibrary.SetScalarParameterValue` "/Game/ChronoSwitch/Materials/Collections/MC_TimeSwap.MC_TimeSwap" "FlashCurve" 1.0)
      (`AudioParameterControllerInterface.SetIntParameter` _ms_switch "Index" 0)
      (`AudioParameterControllerInterface.SetTriggerParameter` _ms_switch "Play")
      (`AudioParameterControllerInterface.SetTriggerParameter` _ms_switch "Trigger Release 2")
      (bind (_direction _timeswap _past) (`Timeline|Timeline` :!label _label_3)
        (:`Update`
          (`KismetMaterialLibrary.SetScalarParameterValue` "/Game/ChronoSwitch/Materials/Collections/MC_TimeSwap.MC_TimeSwap" "Material State" _timeswap)
          (`AudioParameterControllerInterface.SetFloatParameter` _ms_soundscape "Gain 0" _past)
          (`AudioParameterControllerInterface.SetFloatParameter` _ms_soundscape "Gain 1" _timeswap)))
      (else
        (`KismetMaterialLibrary.SetVectorParameterValue` "/Game/ChronoSwitch/Materials/Collections/MC_TimeSwap.MC_TimeSwap" "FlashColor" (`|GetArrayItem` _parametervalue 1))
        (`KismetMaterialLibrary.SetScalarParameterValue` "/Game/ChronoSwitch/Materials/Collections/MC_TimeSwap.MC_TimeSwap" "FlashCurve")
        (`AudioParameterControllerInterface.SetIntParameter` _ms_switch "Index" 1)
        (`AudioParameterControllerInterface.SetTriggerParameter` _ms_switch "Play")
        (`AudioParameterControllerInterface.SetTriggerParameter` _ms_switch "Trigger Release 1")
        (goto _label_3 :!via `Reverse`)))))

(event `Key|E`
  (params (Key :type "Key Structure")))

(event `self.OnVisorStateChangedCosmetic`
  (params (bIsVisorActive :type Boolean))
  ;[1 0.4517 0 0.5] HandleVisorToggle
  (if (not bIsVisorActive)
    (bind (_direction _timeswap _postprocess) (`Timeline|VisorTimeline` :!label _label_4)
      (:`Update`
        (`KismetMaterialLibrary.SetScalarParameterValue` "/Game/ChronoSwitch/Materials/Collections/MC_TimeSwap.MC_TimeSwap" "FullVanish" _timeswap)))
    (else
      (goto _label_4 :!via `Reverse`))))

(event `Key|Q`
  (params (Key :type "Key Structure"))
  (bind _returnvalue (`ChronoSwitchBlueprintLibrary.GetChronoPlayerState` (`GameplayStatics.GetPlayerState` 0)))
  ;[1 0.4517 0 0.5] HandleVisorToggle
  ;;[0 0.3713 1 0.5] Debug
  (:`Pressed`
    (`/Engine/EditorBlueprintResources/StandardMacros.IsValid` _returnvalue
      (:`Is Valid`
        (`/Engine/EditorBlueprintResources/StandardMacros.FlipFlop`
          (:`A`
            (`ChronoSwitchPlayerState.RequestVisorStateChange` _returnvalue false))
          (:`B`
            (`ChronoSwitchPlayerState.RequestVisorStateChange` _returnvalue true)))))))

(event `self.OnAntiPhasingTriggered`
  ;[0 0.3713 1 0.5] Audio
  ;;[1 0.4517 0 0.5] Handle Anti-Phase
  (`GameplayStatics.PlaySound2D` "/Game/ChronoSwitch/Sound/Error/WAV/Error.Error" 1.0 2.0 0.0 null null))

(fn `SetupSounds`
  (bind _ms_soundscape (`self.MS_Soundscape`))
  (bind _returnvalue (`ChronoSwitchBlueprintLibrary.GetChronoPlayerState` (`GameplayStatics.GetPlayerState` 0)))
  (bind _returnvalue_2 (== (`ChronoSwitchPlayerState.GetTimelineID` _returnvalue) 1))
  (`AudioComponent.Play` (`self.MS_Switch`) 0.0)
  (`/Engine/EditorBlueprintResources/StandardMacros.IsValid` _returnvalue
    (:`Is Valid`
      (`AudioParameterControllerInterface.SetFloatParameter` _ms_soundscape "Gain 0" (select `bool` _returnvalue_2 :`false` 1.0 :!type "Float (single-precision)"))
      (`AudioParameterControllerInterface.SetFloatParameter` _ms_soundscape "Gain 1" (select `bool` _returnvalue_2 :`true` 1.0 :!type "Float (single-precision)"))
      (`AudioComponent.Play` _ms_soundscape 0.0))))

(fn `UserConstructionScript`)