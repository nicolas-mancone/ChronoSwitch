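; BP_ProximityDoor is a two-panel sliding door driven by OpenDoor and CloseDoor events, with no proximity detection in these graphs.
; A timeline, with play rate set from OpeningSpeed at BeginPlay, slides the two meshes in opposite directions along local Y, scaled by OpeningOffset.
; Opening plays the timeline and closing reverses it, each behind its own DoOnce with no reset wired, so each fires only once.
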(event `self.ReceiveBeginPlay`
  (`TimelineComponent.SetPlayRate` (`self.DoorAnimation`) (`self.OpeningSpeed`)))

(event `self.OpenDoor`
  (`/Engine/EditorBlueprintResources/StandardMacros.DoOnce` false
    (:`Completed`
      (bind (_direction _door) (`Timeline|DoorAnimation` :!label _label)
        (:`Update`
          (bind _returnvalue (* _door (`self.OpeningOffset`)))
          (`SceneComponent.K2_SetRelativeLocation` (`self.DoorMesh1`) (`KismetMathLibrary.MakeVector` 0.0 _returnvalue) false false)
          (`SceneComponent.K2_SetRelativeLocation` (`self.DoorMesh2`) (`KismetMathLibrary.MakeVector` 0.0 (* _returnvalue -1.0)) false false))))))

(event `self.CloseDoor`
  (`/Engine/EditorBlueprintResources/StandardMacros.DoOnce` false
    (:`Completed`
      (goto _label :!via `Reverse`))))

(fn `UserConstructionScript`)