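; Decontamination room that opens one door pair for an arriving character, then the other once the procedure completes.
; The server sets DoorIsOpen on the first character overlap and in TransitionStart/TransitionEnd, the latter also setting ProcedureComplete.
; Its RepNotify plays or reverses a timeline sliding the pair selected by ProcedureComplete.
; Closing also makes the trigger box block all channels.
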(event `self.ReceiveTransitionStart`
  (`/Engine/EditorBlueprintResources/ActorMacros.Switch Has Authority`
    (:`Authority`
      (set `self.DoorIsOpen` false))))

(event `self.ReceiveTransitionEnd`
  (`/Engine/EditorBlueprintResources/ActorMacros.Switch Has Authority`
    (:`Authority`
      (set `self.ProcedureComplete` true)
      (set `self.DoorIsOpen` true))))

(event `self.OpenDoorBox.OnComponentBeginOverlap`
  (params (OverlappedComponent :type "PrimitiveComponent Object Reference") (OtherActor :type "Actor Object Reference") (OtherComp :type "PrimitiveComponent Object Reference") (OtherBodyIndex :type Integer) (bFromSweep :type Boolean) (SweepResult :type "HitResult Structure (by ref)"))
  ;[0.15 0.1207 0.0045 0.5] Handle Doors
  (`KismetSystemLibrary.IsObjectOfSoftClass` OtherActor "/Script/ChronoSwitch.ChronoSwitchCharacter"
    (:`True`
      (`/Engine/EditorBlueprintResources/StandardMacros.DoOnce` false
        (:`Completed`
          (`/Engine/EditorBlueprintResources/ActorMacros.Switch Has Authority`
            (:`Authority`
              (set `self.DoorIsOpen` true))))))))

(event `OpenDoor`
  (bind _procedurecomplete (`self.ProcedureComplete`))
  (bind _returnvalue (select `bool` _procedurecomplete :`false` (`self.SM_LabDoor03_StaticMeshComponent0`) :`true` (`self.SM_LabDoor6_StaticMeshComponent0`)))
  (bind _returnvalue_2 (select `bool` _procedurecomplete :`false` (`self.SM_LabDoor4_StaticMeshComponent0`) :`true` (`self.SM_LabDoor5_StaticMeshComponent0`)))
  (bind (_relativelocation_x _relativelocation_y _relativelocation_z) (`KismetMathLibrary.BreakVector` (`SceneComponent.RelativeLocation` _returnvalue_2)))
  (bind (_relativelocation_x_2 _relativelocation_y_2 _relativelocation_z_2) (`KismetMathLibrary.BreakVector` (`SceneComponent.RelativeLocation` _returnvalue)))
  ;[0.15 0.1207 0.0045 0.5] Handle Doors
  (bind (_direction _newtrack_0) (`Timeline|OpenDoor1` :!label _label)
    (:`Update`
      (`SceneComponent.K2_SetRelativeLocation` _returnvalue_2 (`KismetMathLibrary.MakeVector` _relativelocation_x (`KismetMathLibrary.MapRangeClamped` _newtrack_0 0.0 1.0 -17.367526 -107.367526) _relativelocation_z) false false)
      (`SceneComponent.K2_SetRelativeLocation` _returnvalue (`KismetMathLibrary.MakeVector` _relativelocation_x_2 (`KismetMathLibrary.MapRangeClamped` _newtrack_0 0.0 1.0 -17.367526 72.632474) _relativelocation_z_2) false false))))

(event `CloseDoor`
  ;[0.15 0.1207 0.0045 0.5] Handle Doors
  (goto _label :!via `Reverse`))

(fn `OnRep_DoorIsOpen`
  (`self.DoorIsOpen`
    (:`then`
      (`self.OpenDoor`))
    (:`else`
      (`self.CloseDoor`)
      (`PrimitiveComponent.SetCollisionResponseToAllChannels` (`self.OpenDoorBox`) "ECR_Block"))))

(fn `UserConstructionScript`)