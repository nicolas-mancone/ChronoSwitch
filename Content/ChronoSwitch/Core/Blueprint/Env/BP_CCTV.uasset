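; BP_CCTV is an environment security camera that swivels to follow the nearer of the two player characters.
; Each Tick it finds the closest player and, within range, converts the look-at rotation into Base's local space, offsets the yaw and clamps it to a half-circle.
; The Scene component eases toward that yaw-only rotation, or more slowly back to neutral when both players are out of range.
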(event `self.ReceiveTick`
  (params (DeltaSeconds :type "Float (single-precision)"))
  (bind _scene (`self.Scene`))
  (bind _scene_2 (`self.Scene`))
  (bind _returnvalue (`self.K2_GetActorLocation` self))
  (bind (_distance _returnvalue_2) (`GameplayStatics.FindNearestActor` _returnvalue (`|MakeArray` (`GameplayStatics.GetPlayerCharacter` 0) (`GameplayStatics.GetPlayerCharacter` 1) :!type "Actor Object Reference")))
  (bind (_returnvalue_roll _returnvalue_pitch _returnvalue_yaw) (`KismetMathLibrary.BreakRotator` (`KismetMathLibrary.InverseTransformRotation` (`SceneComponent.K2_GetComponentToWorld` (`self.Base`)) (`KismetMathLibrary.FindLookAtRotation` _returnvalue (`self.K2_GetActorLocation` _returnvalue_2)))))
  (if (> _distance 1000.0)
    (`SceneComponent.K2_SetRelativeRotation` _scene_2 (`KismetMathLibrary.RInterpTo` (`SceneComponent.RelativeRotation` _scene_2) (struct) DeltaSeconds 2.0) false false)
    (else
      (`SceneComponent.K2_SetRelativeRotation` _scene (`KismetMathLibrary.RInterpTo` (`SceneComponent.RelativeRotation` _scene) (`KismetMathLibrary.MakeRotator` 0.0 0.0 (`KismetMathLibrary.ClampAngle` (- _returnvalue_yaw 90.0) -90.0 90.0)) DeltaSeconds 8.0) false false))))

(fn `UserConstructionScript`)