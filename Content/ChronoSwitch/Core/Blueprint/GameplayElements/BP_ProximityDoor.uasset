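; BP_ProximityDoor is a two-panel sliding door that opens and closes through OpenDoor and CloseDoor events, each gated by a DoOnce.
; A DoorAnimation timeline moves both meshes in opposite directions along local Y, playing to open and reversing to close.
; DoorComponent supplies the slide offset and the timeline play rate, which is set on BeginPlay.
; Each event also plays the MSDoorOpen sound with an Open or Close trigger.
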(event `self.ReceiveBeginPlay`
  (`TimelineComponent.SetPlayRate` (`self.DoorAnimation`) (`DoorComponent.OpeningSpeed` (`self.DoorComponent`))))

(event `self.OpenDoor`
  (bind _ms_dooropen (`self.MS_DoorOpen`))
  (`/Engine/EditorBlueprintResources/StandardMacros.DoOnce` false
    (:`Completed`
      (`AudioComponent.Play` _ms_dooropen 0.0)
      (`AudioParameterControllerInterface.SetTriggerParameter` _ms_dooropen "Open")
      (bind (_direction _door) (`Timeline|DoorAnimation` :!label _label)
        (:`Update`
          (bind _returnvalue (* _door (`DoorComponent.OpeningOffset` (`self.DoorComponent`))))
          (`SceneComponent.K2_SetRelativeLocation` (`self.DoorMesh1`) (`KismetMathLibrary.MakeVector` 0.0 _returnvalue) false false)
          (`SceneComponent.K2_SetRelativeLocation` (`self.DoorMesh2`) (`KismetMathLibrary.MakeVector` 0.0 (* _returnvalue -1.0)) false false))))))

(event `self.CloseDoor`
  (bind _ms_dooropen (`self.MS_DoorOpen`))
  (`/Engine/EditorBlueprintResources/StandardMacros.DoOnce` false
    (:`Completed`
      (`AudioComponent.Play` _ms_dooropen 0.0)
      (`AudioParameterControllerInterface.SetTriggerParameter` _ms_dooropen "Close")
      (goto _label :!via `Reverse`))))

(fn `UserConstructionScript`)