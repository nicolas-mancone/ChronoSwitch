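; BP_PairedProximityDoors is a pair of sliding doors that open and close together through OpenDoor and CloseDoor events, whose callers are outside this graph.
; A shared timeline, its play rate set from DoorComponent's opening speed, slides the two mesh sets in opposite directions along local Y by the component's offset.
; Each event passes a DoOnce with no reset wired, triggers an open or close sound, then plays or reverses the timeline.
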(event `self.ReceiveBeginPlay`
  (`TimelineComponent.SetPlayRate` (`self.DoorTimeline`) (`DoorComponent.OpeningSpeed` (`self.DoorComponent`))))

(event `self.OpenDoor`
  (bind _ms_dooropen (`self.MS_DoorOpen`))
  (`/Engine/EditorBlueprintResources/StandardMacros.DoOnce` false
    (:`Completed`
      (`AudioComponent.Play` _ms_dooropen 0.0)
      (`AudioParameterControllerInterface.SetTriggerParameter` _ms_dooropen "Open")
      (bind (_direction _doorvalue) (`Timeline|DoorTimeline` :!label _label)
        (:`Update`
          (`|ExecutionSequence`
            (:`then_0`
              (bind _returnvalue (* _doorvalue (`DoorComponent.OpeningOffset` (`self.DoorComponent`))))
              (`SceneComponent.K2_SetRelativeLocation` (`self.DoorMesh1D1`) (`KismetMathLibrary.MakeVector` 0.0 _returnvalue) false false)
              (`SceneComponent.K2_SetRelativeLocation` (`self.DoorMesh1D2`) (`KismetMathLibrary.MakeVector` 0.0 _returnvalue) false false))
            (:`then_1`
              (bind _returnvalue_2 (* _returnvalue -1.0))
              (`SceneComponent.K2_SetRelativeLocation` (`self.DoorMesh2D1`) (`KismetMathLibrary.MakeVector` 0.0 _returnvalue_2) false false)
              (`SceneComponent.K2_SetRelativeLocation` (`self.DoorMesh2D2`) (`KismetMathLibrary.MakeVector` 0.0 _returnvalue_2) false false))))))))

(event `self.CloseDoor`
  (bind _ms_dooropen (`self.MS_DoorOpen`))
  (`/Engine/EditorBlueprintResources/StandardMacros.DoOnce` false
    (:`Completed`
      (`AudioComponent.Play` _ms_dooropen 0.0)
      (`AudioParameterControllerInterface.SetTriggerParameter` _ms_dooropen "Close")
      (goto _label :!via `Reverse`))))

(fn `UserConstructionScript`)