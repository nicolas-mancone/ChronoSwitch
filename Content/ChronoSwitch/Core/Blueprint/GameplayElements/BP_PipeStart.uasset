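; BP_PipeStart is a gameplay element that animates a given actor into a slot, then activates itself.
; MoveActorinPlace runs a half-speed timeline that blends the actor's location and rotation toward Slot, then a second timeline that inserts it into SlotInterior.
; Each phase fires a one-shot sound through DoOnce.
; When insertion finishes, it hides the actor's FutureMesh and calls ActivateObject after a short delay.
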(event `self.ReceiveBeginPlay`
  (`TimelineComponent.SetPlayRate` (`self.MovementTimeline`) 0.5))

(event `self.MoveActorInPlace`
  (params (MovingActor :type "FuturePhysicsTimelineActor Object Reference"))
  (bind (_returnvalue_location _returnvalue_rotation _returnvalue_scale) (`KismetMathLibrary.BreakTransform` (`self.GetTransform` MovingActor)))
  (bind (_returnvalue_location_2 _returnvalue_rotation_2 _returnvalue_scale_2) (`KismetMathLibrary.BreakTransform` (`self.GetTransform` MovingActor)))
  (bind (_returnvalue_location_3 _returnvalue_rotation_3) (`KismetMathLibrary.BreakTransform` (`SceneComponent.K2_GetComponentToWorld` (`self.Slot`))))
  (bind (_returnvalue_location_4 _returnvalue_rotation_4) (`KismetMathLibrary.BreakTransform` (`SceneComponent.K2_GetComponentToWorld` (`self.SlotInterior`))))
  (bind (_direction _newtrack_0) (`Timeline|MovementTimeline`)
    (:`Update`
      (if (>= _newtrack_0 0.2)
        (`/Engine/EditorBlueprintResources/StandardMacros.DoOnce` false
          (:`Completed`
            (`AudioComponent.Play` (`self.Audio1`) 0.0))))
      (`self.K2_SetActorTransform` MovingActor (`KismetMathLibrary.TLerp` (`KismetMathLibrary.MakeTransform` _returnvalue_location _returnvalue_rotation _returnvalue_scale) (`KismetMathLibrary.MakeTransform` _returnvalue_location_3 _returnvalue_rotation_3 _returnvalue_scale) _newtrack_0) false false))
    (:`Finished`
      (bind (_direction_2 _newtrack_0_2) (`Timeline|InsertionValue`)
        (:`Update`
          (`self.K2_SetActorTransform` MovingActor (`KismetMathLibrary.TLerp` (`KismetMathLibrary.MakeTransform` _returnvalue_location_2 _returnvalue_rotation_2 _returnvalue_scale_2) (`KismetMathLibrary.MakeTransform` _returnvalue_location_4 _returnvalue_rotation_4 _returnvalue_scale_2) _newtrack_0_2) false false)
          (if (>= _newtrack_0_2 0.01)
            (`/Engine/EditorBlueprintResources/StandardMacros.DoOnce` false
              (:`Completed`
                (`AudioComponent.Play` (`self.Audio`) 0.0)))))
        (:`Finished`
          (`SceneComponent.SetVisibility` (`TimelineBaseActor.FutureMesh` MovingActor) false true)
          (`KismetSystemLibrary.Delay` 0.5)
          (`self.ActivateObject`))))))

(fn `UserConstructionScript`)