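; BP_PipeEnd is the outlet of a pipe that ejects a physics actor, apparently a powercell, when activated.
; OnActivation teleports the actor to SlotInterior and shows its FutureMesh, then the OutMovement timeline lerps it from its current transform toward Slot, preserving scale.
; A DoOnce with no reset plays the exit sound partway through.
; On finish, collision and physics simulation on both Future and Past meshes switch on.
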(event `self.OnActivation`
  (params (NewPhysicsActor :type "FuturePhysicsTimelineActor Object Reference"))
  (bind (_returnvalue_location _returnvalue_rotation _returnvalue_scale) (`KismetMathLibrary.BreakTransform` (`self.GetTransform` NewPhysicsActor)))
  (bind (_returnvalue_location_2 _returnvalue_rotation_2 _returnvalue_scale_2) (`KismetMathLibrary.BreakTransform` (`self.GetTransform` NewPhysicsActor)))
  (bind (_returnvalue_location_3 _returnvalue_rotation_3) (`KismetMathLibrary.BreakTransform` (`SceneComponent.K2_GetComponentToWorld` (`self.SlotInterior`))))
  (bind (_returnvalue_location_4 _returnvalue_rotation_4) (`KismetMathLibrary.BreakTransform` (`SceneComponent.K2_GetComponentToWorld` (`self.Slot`))))
  (`self.K2_SetActorTransform` NewPhysicsActor (`KismetMathLibrary.MakeTransform` _returnvalue_location_3 _returnvalue_rotation_3 _returnvalue_scale) false true)
  (`SceneComponent.SetVisibility` (`TimelineBaseActor.FutureMesh` NewPhysicsActor) true false)
  (bind (_direction _value) (`Timeline|OutMovement`)
    (:`Update`
      (`self.K2_SetActorTransform` NewPhysicsActor (`KismetMathLibrary.TLerp` (`KismetMathLibrary.MakeTransform` _returnvalue_location_2 _returnvalue_rotation_2 _returnvalue_scale_2) (`KismetMathLibrary.MakeTransform` _returnvalue_location_4 _returnvalue_rotation_4 _returnvalue_scale_2) _value) false false)
      (if (>= _value 0.2)
        (`/Engine/EditorBlueprintResources/StandardMacros.DoOnce` false
          (:`Completed`
            (`AudioComponent.Play` (`self.MSS_Powercell_Out`) 0.0)))))
    (:`Finished`
      (`self.SetActorEnableCollision` NewPhysicsActor true)
      (`PrimitiveComponent.SetSimulatePhysics` (`TimelineBaseActor.FutureMesh` NewPhysicsActor) true)
      (`PrimitiveComponent.SetSimulatePhysics` (`TimelineBaseActor.PastMesh` NewPhysicsActor) true))))

(fn `UserConstructionScript`)