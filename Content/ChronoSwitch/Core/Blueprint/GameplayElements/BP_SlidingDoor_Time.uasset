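; Sliding door that opens and closes and changes its visible mesh with the player's timeline.
; A timeline, paced by the door component's opening speed, slides the door mesh along Y by the component's offset and reverses to close.
; Open and close sounds fire only on authority through audio trigger parameters.
; A timeline observer binding supports swapping present and past meshes, briefly overlapping both before hiding the old one.
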(event `self.ReceiveBeginPlay`
  (`TimelineComponent.SetPlayRate` (`self.ManageDoor`) (`DoorComponent.OpeningSpeed` (`self.DoorComponent`)))
  (add `TimelineObserverComponent.OnPlayerTimelineStateUpdated` (`self.TimelineObserver`) (`|CreateDelegate` :!event `HandleTimeline`)))

(event `PlaySound`
  (bind _audio (`self.Audio`))
  (`AudioComponent.Play` _audio 0.0)
  (`AudioParameterControllerInterface.SetTriggerParameter` _audio "Open"))

(event `self.OpenDoor`
  (`/Engine/EditorBlueprintResources/ActorMacros.Switch Has Authority`
    (:`Authority`
      (`self.PlaySound`)
      (bind (_direction _newtrack_0) (`Timeline|ManageDoor` :!label _label)
        (:`Update`
          (`SceneComponent.K2_SetRelativeLocation` (`self.DoorMesh`) (`KismetMathLibrary.MakeVector` 0.0 (* _newtrack_0 (`DoorComponent.OpeningOffset` (`self.DoorComponent`)))) false false))))
    (:`Remote`
      (goto _label))))

(event `self.CloseDoor`
  (`/Engine/EditorBlueprintResources/ActorMacros.Switch Has Authority`
    (:`Authority`
      (`self.PlaySoundClose`)
      (goto _label :!via `Reverse`))
    (:`Remote`
      (goto _label :!via `Reverse`))))

(event `PlaySoundClose`
  (bind _audio (`self.Audio`))
  (`AudioComponent.Play` _audio 0.0)
  (`AudioParameterControllerInterface.SetTriggerParameter` _audio "Close"))

(event `HandleTimeline`
  (params (PlayerTimelineID :type Byte) (bIsVisorActive :type Boolean))
  (if (== PlayerTimelineID 1)
    (`SceneComponent.SetHiddenInGame` (`self.DoorMesh`) false false)
    (`KismetSystemLibrary.Delay` 0.7)
    (`SceneComponent.SetHiddenInGame` (`self.DoorPast`) true false)
    (else
      (`SceneComponent.SetHiddenInGame` (`self.DoorPast`) false false)
      (`KismetSystemLibrary.Delay` 0.7)
      (`SceneComponent.SetHiddenInGame` (`self.DoorMesh`) true false))))

(fn `UserConstructionScript`)