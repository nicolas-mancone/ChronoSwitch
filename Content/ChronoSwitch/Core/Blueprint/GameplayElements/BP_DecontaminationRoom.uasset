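; Two-player decontamination airlock that masks a transition between an entry and an exit door.
; Overlap boxes count players to open and close the entry; the server sets DoorIsOpen, whose RepNotify drives the sliding-door timeline and audio.
; TransitionStart shuts the door and runs timed water, then smoke Niagara and MetaSound phases, each scaled from MinTransitionDuration.
; TransitionEnd sets ProcedureComplete, switching door logic to the exit, and opens it.
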(event `self.ReceiveBeginPlay`
  (set `self.NiagaraRains` (`|MakeArray` (`self.WaterEffect`) (`self.WaterEffect1`) (`self.WaterEffect2`) (`self.WaterEffect3`) (`self.WaterEffect4`) (`self.WaterEffect5`) (`self.WaterEffect6`) (`self.WaterEffect7`)))
  (set `self.NiagaraSmokes` (`|MakeArray` (`self.SmokeEffect`) (`self.SmokeEffect1`) (`self.SmokeEffect2`) (`self.SmokeEffect3`) (`self.SmokeEffect4`) (`self.SmokeEffect5`) (`self.SmokeEffect6`) (`self.SmokeEffect7`) (`self.SmokeEffect8`) (`self.SmokeEffect9`) (`self.SmokeEffect10`) (`self.SmokeEffect11`) (`self.SmokeEffect12`) (`self.SmokeEffect13`) (`self.SmokeEffect14`) (`self.SmokeEffect15`))))

(event `self.ReceiveTransitionStart`
  ;[0.02691 0.1823 1 0.5] StartTransition, close door, start niagara water and sound
  (`|ExecutionSequence`
    (:`then_0`
      (`/Engine/EditorBlueprintResources/ActorMacros.Switch Has Authority`
        (:`Authority`
          (set `self.DoorIsOpen` false))))
    (:`then_1`
      (for _array_element (`self.NiagaraRains`)
        (`ActorComponent.ToggleActive` _array_element))
      (`AudioComponent.Play` (`self.MSS_DecontanimWater`) 0.0)
      (bind _returnvalue (`KismetSystemLibrary.K2_SetTimerDelegate` (`|CreateDelegate` :!event `OnWaterFinished`) (/ (`self.MinTransitionDuration`) 2.2)))
      (set `self.WaterTimer` _returnvalue))))

(event `OnWaterFinished`
  ;[1 0.562 0.03745 0.5] Deactivate water niagara and sound, start smoke niagara and sound
  (for _array_element (`self.NiagaraRains`)
    (`ActorComponent.ToggleActive` _array_element))
  (`AudioParameterControllerInterface.SetTriggerParameter` (`self.MSS_DecontanimWater`) "Stop")
  (for _array_element_2 (`self.NiagaraSmokes`)
    (`ActorComponent.ToggleActive` _array_element_2))
  (`AudioComponent.Play` (`self.MSS_DecontanimSmoke`) 0.0)
  (bind _returnvalue (`KismetSystemLibrary.K2_SetTimerDelegate` (`|CreateDelegate` :!event `OnSmokeFinished`) (/ (`self.MinTransitionDuration`) 2.2)))
  (set `self.SmokeTimer` _returnvalue))

(event `OnSmokeFinished`
  ;[0.02691 0.1823 1 0.5] Stop Smoke Niagara and Sound
  (for _array_element (`self.NiagaraSmokes`)
    (`ActorComponent.ToggleActive` _array_element))
  (`AudioParameterControllerInterface.SetTriggerParameter` (`self.MSS_DecontanimSmoke`) "Stop"))

(event `self.ReceiveTransitionEnd`
  ;[1 0.562 0.03745 0.5] End Transition
  (`/Engine/EditorBlueprintResources/ActorMacros.Switch Has Authority`
    (:`Authority`
      (set `self.ProcedureComplete` true)
      (set `self.DoorIsOpen` true)
      (`KismetSystemLibrary.K2_ClearAndInvalidateTimerHandle` (`self.WaterTimer`))
      (`KismetSystemLibrary.K2_ClearAndInvalidateTimerHandle` (`self.SmokeTimer`)))))

(event `self.OpenDoorBox.OnComponentBeginOverlap`
  (params (OverlappedComponent :type "PrimitiveComponent Object Reference") (OtherActor :type "Actor Object Reference") (OtherComp :type "PrimitiveComponent Object Reference") (OtherBodyIndex :type Integer) (bFromSweep :type Boolean) (SweepResult :type "HitResult Structure (by ref)"))
  ;[0.02691 0.1823 1 0.5] OpenDoorLogic
  (`KismetSystemLibrary.IsObjectOfSoftClass` OtherActor "/Script/ChronoSwitch.ChronoSwitchCharacter"
    (:`True`
      (`self.DoublePlayerRequired`
        (:`then`
          (bind _result (`/Engine/EditorBlueprintResources/StandardMacros.IncrementInt` (`self.PlayerIndex`))
            (:`  `
              (if (== _result 2)
                (`/Engine/EditorBlueprintResources/StandardMacros.DoOnce` false :!label _label
                  (:`Completed`
                    (`/Engine/EditorBlueprintResources/ActorMacros.Switch Has Authority`
                      (:`Authority`
                        (set `self.DoorIsOpen` true)))))))))
        (:`else`
          (goto _label))))))

(event `self.OpenDoorBox.OnComponentEndOverlap`
  (params (OverlappedComponent :type "PrimitiveComponent Object Reference") (OtherActor :type "Actor Object Reference") (OtherComp :type "PrimitiveComponent Object Reference") (OtherBodyIndex :type Integer))
  ;[0.02691 0.1823 1 0.5] OpenDoorLogic
  (`KismetSystemLibrary.IsObjectOfSoftClass` OtherActor "/Script/ChronoSwitch.ChronoSwitchCharacter"
    (:`True`
      (`self.DoublePlayerRequired`
        (:`then`
          (`/Engine/EditorBlueprintResources/StandardMacros.DecrementInt` (`self.PlayerIndex`)))
        (:`else`)))))

(event `OpenDoor`
  (bind _procedurecomplete (`self.ProcedureComplete`))
  (bind _returnvalue (select `bool` _procedurecomplete :`false` (`self.SM_LabDoor03_StaticMeshComponent0`) :`true` (`self.SM_LabDoor6_StaticMeshComponent0`)))
  (bind _returnvalue_2 (select `bool` _procedurecomplete :`false` (`self.SM_LabDoor4_StaticMeshComponent0`) :`true` (`self.SM_LabDoor5_StaticMeshComponent0`)))
  (bind _returnvalue_3 (select `bool` _procedurecomplete :`false` (`self.Door1`) :`true` (`self.Door2`)))
  (bind (_relativelocation_x _relativelocation_y _relativelocation_z) (`KismetMathLibrary.BreakVector` (`SceneComponent.RelativeLocation` _returnvalue_2)))
  (bind (_relativelocation_x_2 _relativelocation_y_2 _relativelocation_z_2) (`KismetMathLibrary.BreakVector` (`SceneComponent.RelativeLocation` _returnvalue)))
  ;[1 0.562 0.03745 0.5] Handle Doors
  (`AudioComponent.Play` _returnvalue_3 0.0)
  (`AudioParameterControllerInterface.SetTriggerParameter` _returnvalue_3 "Open")
  (bind (_direction _newtrack_0) (`Timeline|OpenDoor1` :!label _label_2)
    (:`Update`
      (`SceneComponent.K2_SetRelativeLocation` _returnvalue_2 (`KismetMathLibrary.MakeVector` _relativelocation_x (`KismetMathLibrary.MapRangeClamped` _newtrack_0 0.0 1.0 -17.367526 -107.367526) _relativelocation_z) false false)
      (`SceneComponent.K2_SetRelativeLocation` _returnvalue (`KismetMathLibrary.MakeVector` _relativelocation_x_2 (`KismetMathLibrary.MapRangeClamped` _newtrack_0 0.0 1.0 -17.367526 72.632474) _relativelocation_z_2) false false))))

(event `CloseDoor`
  (bind _returnvalue (select `bool` (`self.ProcedureComplete`) :`false` (`self.Door1`) :`true` (`self.Door2`)))
  ;[1 0.562 0.03745 0.5] Handle Doors
  (`AudioComponent.Play` _returnvalue 0.0)
  (`AudioParameterControllerInterface.SetTriggerParameter` _returnvalue "Close")
  (goto _label_2 :!via `Reverse`))

(event `self.CloseDoorBox.OnComponentBeginOverlap`
  (params (OverlappedComponent :type "PrimitiveComponent Object Reference") (OtherActor :type "Actor Object Reference") (OtherComp :type "PrimitiveComponent Object Reference") (OtherBodyIndex :type Integer) (bFromSweep :type Boolean) (SweepResult :type "HitResult Structure (by ref)"))
  (bind _playersarray (`self.PlayersArray`))
  (bind _asbp_chrono_switch_character (cast `/Game/ChronoSwitch/Core/Characters/BP_ChronoSwitchCharacter` OtherActor))
  (`KismetArrayLibrary.Array_AddUnique` _playersarray _asbp_chrono_switch_character)
  (if (== (`KismetArrayLibrary.Array_Length` _playersarray) 2)
    (`/Engine/EditorBlueprintResources/StandardMacros.DoOnce` false
      (:`Completed`
        (`/Engine/EditorBlueprintResources/ActorMacros.Switch Has Authority`
          (:`Authority`
            (set `self.DoorIsOpen` false)))))))

(event `self.DoorBoxCheck.OnComponentBeginOverlap`
  (params (OverlappedComponent :type "PrimitiveComponent Object Reference") (OtherActor :type "Actor Object Reference") (OtherComp :type "PrimitiveComponent Object Reference") (OtherBodyIndex :type Integer) (bFromSweep :type Boolean) (SweepResult :type "HitResult Structure (by ref)"))
  (bind _asbp_chrono_switch_character (cast `/Game/ChronoSwitch/Core/Characters/BP_ChronoSwitchCharacter` OtherActor))
  (`KismetArrayLibrary.Array_RemoveItem` (`self.PlayersArray`) _asbp_chrono_switch_character))

(fn `OnRep_DoorIsOpen`
  (`self.DoorIsOpen`
    (:`then`
      (`self.OpenDoor`))
    (:`else`
      (`self.CloseDoor`)
      (`PrimitiveComponent.SetCollisionResponseToAllChannels` (`self.OpenDoorBox`) "ECR_Block"))))

(fn `UserConstructionScript`)