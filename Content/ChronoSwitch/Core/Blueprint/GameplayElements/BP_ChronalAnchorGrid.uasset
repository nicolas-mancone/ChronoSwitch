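; Chronal anchor grid gameplay element with a barrier mesh tinted by the timeline it targets on entry and an audio cue for crossings.
; On BeginPlay it creates a dynamic material and sets its color for Past, Future or None from the entering-crossing settings.
; ManageSoundonCrossing calls PlaySound only on authority to play the crossing audio.
; The crossing detection and timeline-forcing logic are not in this graph.
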(event `self.ReceiveBeginPlay`
  (bind _barriermesh (`self.BarrierMesh`))
  (bind _barriercolors (`self.BarrierColors`))
  (bind _returnvalue (`PrimitiveComponent.CreateDynamicMaterialInstance` _barriermesh 0 (`PrimitiveComponent.GetMaterial` _barriermesh 0) "None"))
  (set `self.BarierMaterialInstance` _returnvalue)
  (bind _bariermaterialinstance (`self.BarierMaterialInstance`)
    (:`then`
      (`MaterialInstanceDynamic.SetVectorParameterValue` _bariermaterialinstance "Color" (select `EForcedTimeline` (`.TargetForcedTimeline` (break `CrossingSettings` (`self.EnteringCrossingSettings`))) :`Past` (`|GetArrayItem` _barriercolors) :`Future` (`|GetArrayItem` _barriercolors 1) :`None` (`|GetArrayItem` _barriercolors 2))))
    (:`else`)))

(event `self.ManageSoundOnCrossing`
  (`/Engine/EditorBlueprintResources/ActorMacros.Switch Has Authority`
    (:`Authority`
      (`self.PlaySound`))))

(event `PlaySound`
  (`AudioComponent.Play` (`self.Crossing Audio`) 0.0))

(fn `UserConstructionScript`)