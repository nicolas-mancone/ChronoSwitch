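; BP_EndingZone is a trigger volume that starts the game's ending once two ChronoSwitch characters are inside.
; The server tracks overlapping characters, then fires Ending and sets the time switch mode to None.
; Ending blocks player 0's movement, mutes both soundscapes, plays the ending theme and, if Ball is valid, stops its audio and shows credits after a delay.
; A TeleportPlayers event alternating characters between two heights has no live caller.
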(event `self.Box.OnComponentBeginOverlap`
  (params (OverlappedComponent :type "PrimitiveComponent Object Reference") (OtherActor :type "Actor Object Reference") (OtherComp :type "PrimitiveComponent Object Reference") (OtherBodyIndex :type Integer) (bFromSweep :type Boolean) (SweepResult :type "HitResult Structure (by ref)"))
  (bind _returnvalue (`ChronoSwitchBlueprintLibrary.GetChronoGameState`))
  (bind _charactersindex (`self.CharactersIndex`))
  (`/Engine/EditorBlueprintResources/ActorMacros.Switch Has Authority`
    (:`Authority`
      (cast `/Game/ChronoSwitch/Core/Characters/BP_ChronoSwitchCharacter` OtherActor)
      (`KismetArrayLibrary.Array_AddUnique` (`self.As BP Chrono Switch Character`))
      (`/Engine/EditorBlueprintResources/StandardMacros.IncrementInt` _charactersindex
        (:`  `
          (if (== _charactersindex 2)
            (`self.Ending`)
            (`/Engine/EditorBlueprintResources/StandardMacros.IsValid` _returnvalue
              (:`Is Valid`
                (`ChronoSwitchGameState.SetTimeSwitchMode` _returnvalue "None")))))))))

(event `self.Box.OnComponentEndOverlap`
  (params (OverlappedComponent :type "PrimitiveComponent Object Reference") (OtherActor :type "Actor Object Reference") (OtherComp :type "PrimitiveComponent Object Reference") (OtherBodyIndex :type Integer))
  (`/Engine/EditorBlueprintResources/ActorMacros.Switch Has Authority`
    (:`Authority`
      (bind _asbp_chrono_switch_character (cast `/Game/ChronoSwitch/Core/Characters/BP_ChronoSwitchCharacter` OtherActor))
      (`/Engine/EditorBlueprintResources/StandardMacros.DecrementInt` (`self.CharactersIndex`)
        (:`  `
          (`KismetArrayLibrary.Array_RemoveItem` (`self.As BP Chrono Switch Character`) _asbp_chrono_switch_character))))))

(event `Ending`
  (bind _returnvalue (`GameplayStatics.GetPlayerController` 0))
  (bind _ball (`self.ball`))
  (`Controller.SetIgnoreMoveInput` _returnvalue true)
  (bind _asbp_chrono_switch_character (cast `/Game/ChronoSwitch/Core/Characters/BP_ChronoSwitchCharacter` (`Controller.K2_GetPawn` _returnvalue)))
  (`AudioComponent.AdjustVolume` (`/Game/ChronoSwitch/Core/Characters/BP_ChronoSwitchCharacter.MS_SoundscapeFuture` _asbp_chrono_switch_character) 0.0 0.0 "Linear")
  (`AudioComponent.AdjustVolume` (`/Game/ChronoSwitch/Core/Characters/BP_ChronoSwitchCharacter.MS_Soundscape` _asbp_chrono_switch_character) 0.0 0.0 "Linear")
  (`GameplayStatics.PlaySound2D` "/Game/ChronoSwitch/Sound/Chronoswitch_ending_theme.Chronoswitch_ending_theme" 1.0 1.0 0.0 null null)
  (`/Engine/EditorBlueprintResources/StandardMacros.IsValid` _ball
    (:`Is Valid`
      (`KismetSystemLibrary.Delay` 6.0)
      (`AudioComponent.Stop` (`AmbientSound.AudioComponent` _ball))
      (bind _returnvalue_2 (`|CreateWidget` "/Game/ChronoSwitch/Core/UI/WBP_Credits.WBP_Credits_C" _returnvalue))
      (`UserWidget.AddToViewport` _returnvalue_2 0))))

(event `TeleportPlayers`
  (set `self.IsFuture` (not (`self.IsFuture`)))
  (for _array_element (`self.As BP Chrono Switch Character`)
    (`/Engine/EditorBlueprintResources/StandardMacros.IsValid` _array_element
      (:`Is Valid`
        (if (`self.IsFuture`)
          (`self.K2_SetActorLocation` _array_element (0.0 0.0 -4401.999999) false true)
          (else
            (`self.K2_SetActorLocation` _array_element (0.0 0.0 88.000004) false true))))))
  (`KismetSystemLibrary.K2_SetTimerDelegate` (`|CreateDelegate` :!event `TeleportPlayers`) 0.0 false false (`KismetMathLibrary.RandomFloatInRange` 1.5 4.0)))

(fn `UserConstructionScript`)