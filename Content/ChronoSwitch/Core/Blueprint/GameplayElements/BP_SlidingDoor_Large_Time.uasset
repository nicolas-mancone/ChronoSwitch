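; Large two-panel sliding door that changes its visible meshes with the player's timeline.
; Open and close events, each behind a DoOnce, trigger a sound and play or reverse a timeline that slides the panels in opposite directions, using speed and offset from DoorComponent.
; TimelineObserver updates swap the main and past door meshes, showing the new set immediately and hiding the old after a short overlap delay.
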(event `self.ReceiveBeginPlay`
  (`TimelineComponent.SetPlayRate` (`self.DoorAnimation`) (`DoorComponent.OpeningSpeed` (`self.DoorComponent`)))
  (add `TimelineObserverComponent.OnPlayerTimelineStateUpdated` (`self.TimelineObserver`) (`|CreateDelegate` :!event `HandleTimeline`)))

(event `self.OpenDoor`
  (bind _ms_dooropen (`self.MS_DoorOpen`))
  (`/Engine/EditorBlueprintResources/StandardMacros.DoOnce` false
    (:`Completed`
      (`AudioComponent.Play` _ms_dooropen 0.0)
      (`AudioParameterControllerInterface.SetTriggerParameter` _ms_dooropen "Open")
      (bind (_direction _door) (`Timeline|DoorAnimation` :!label _label)
        (:`Update`
          (bind _returnvalue (* _door (`DoorComponent.OpeningOffset` (`self.DoorComponent`))))
          (`SceneComponent.K2_SetRelativeLocation` (`self.DoorMesh`) (`KismetMathLibrary.MakeVector` 0.0 _returnvalue) false false)
          (`SceneComponent.K2_SetRelativeLocation` (`self.Door1`) (`KismetMathLibrary.MakeVector` 0.0 (* _returnvalue -1.0)) false false))))))

(event `self.CloseDoor`
  (bind _ms_dooropen (`self.MS_DoorOpen`))
  (`/Engine/EditorBlueprintResources/StandardMacros.DoOnce` false
    (:`Completed`
      (`AudioComponent.Play` _ms_dooropen 0.0)
      (`AudioParameterControllerInterface.SetTriggerParameter` _ms_dooropen "Close")
      (goto _label :!via `Reverse`))))

(event `HandleTimeline`
  (params (PlayerTimelineID :type Byte) (bIsVisorActive :type Boolean))
  (if (== PlayerTimelineID 1)
    (`SceneComponent.SetHiddenInGame` (`self.DoorMesh`) false false)
    (`SceneComponent.SetHiddenInGame` (`self.Door1`) false false)
    (`KismetSystemLibrary.Delay` 0.7)
    (`SceneComponent.SetHiddenInGame` (`self.DoorPast`) true false)
    (`SceneComponent.SetHiddenInGame` (`self.DoorPast2`) true false)
    (else
      (`SceneComponent.SetHiddenInGame` (`self.DoorPast`) false false)
      (`SceneComponent.SetHiddenInGame` (`self.DoorPast2`) false false)
      (`KismetSystemLibrary.Delay` 0.7)
      (`SceneComponent.SetHiddenInGame` (`self.DoorMesh`) true false)
      (`SceneComponent.SetHiddenInGame` (`self.Door1`) true false))))

(fn `UserConstructionScript`)