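; Player controller Blueprint for ChronoSwitch whose live event graph is empty, holding unwired test logic for switching timelines.
; That logic toggles a Future flag, requests the timeline change on ChronoSwitchPlayerState and sets flash parameters in MC_TimeSwap.
; A Timeline, played or reversed, drives the material state and modulates MSSwitch sound bandwidth, cutoff and gain before a release trigger.
; A separate macro sets filter parameters and triggers a delayed release.
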(event `self.ReceiveBeginPlay`)

(fn `UserConstructionScript`)